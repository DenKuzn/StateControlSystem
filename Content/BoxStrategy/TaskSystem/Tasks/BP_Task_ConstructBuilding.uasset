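; Construction task for the BoxStrategy task system, tracking production points gathered toward raising a building.
; It takes its required amount from ConstructBuilding settings on initialization, closing itself if the cast fails.
; Incoming points are clamped and accumulated, broadcasting updates until the task completes, with progress exposed as gathered over required.
; Offered units receive an assignment message only while a work place is available.
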(event Custom|Event_AddProductionPoint
  (params (ProductedPoint :type Float%20%28double-precision%29))
  (Development|PrintString "Got points")
  (Variables|Default|SetGatheredProductionPoints (+ (Variables|Default|GetGatheredProductionPoints) (Math|Float|Clamp(Float) ProductedPoint 0.0 (Math|Conversions|ToFloat(Integer) (Variables|Default|GetRequiredProductionPoints)))))
  (if (> (Variables|Default|GetRequiredProductionPoints) (Variables|Default|GetGatheredProductionPoints))
    (Default|CallOnTaskWasUpdated)
    (else
      (CallFunction|CompleteTask))))

(event EventTryAssignUnitstoTask
  (params (UnitsToAssign :type Array%20of%20Object%20Object%20References))
  (for _array_element UnitsToAssign
    (bind _returnvalue (CallFunction|CanUnitWorkonThisTask _array_element))
    (if _returnvalue
      (Class|SearchingWorkObjectInterface|NewTaskAssigned(Message) _array_element self))))

(event EventInitializeTaskwithSettings
  (params (Settings :type BP%20Task%20Settings%20Base%20Object%20Reference))
  (bind _asbp_task_settings_construct_building (Utilities|Casting|CastToBP_TaskSettings_ConstructBuilding Settings)
    (:then
      (Variables|Default|SetRequiredProductionPoints (Variables|/Game/BoxStrategy/TaskSystem/Tasks/Settings/BP_TaskSettings_ConstructBuilding.BP_TaskSettings_ConstructBuilding_C|GetRequestedProductionAmount _asbp_task_settings_construct_building))
      (Default|CallOnTaskInitializationFinished))
    (:CastFailed
      (CallFunction|BoxStrategyPrintStringError self "Event_InitializeTashWithSettings" "Cannot cast to CunstrctBuilding Settings")
      (CallFunction|CloseThisTask))))

(fn GetTaskProgressPercent
  (return (/ (Variables|Default|GetGatheredProductionPoints) (Variables|Default|GetRequiredProductionPoints))))

(fn CanUnitWorkonThisTask
  (params (TaskSearchingUnit :type Object%20Object%20Reference))
  (return (CallFunction|IsAvailableWorkPlace)))