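; Strategy-game task that has units deliver a requested set of resources to fulfil a demand taken from its task settings.
; Three per-resource maps track demand, reserved and delivered amounts; units are offered the task while any demand remains unreserved.
; Reserving clamps to the remainder and registers a worker; delivering moves reserved to delivered, removes the worker and completes the task once demand is met.
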(event EventInitializeTaskwithSettings
  (params (Settings :type BP%20Task%20Settings%20Base%20Object%20Reference))
  (bind _asbp_task_settings_resurce_delivery (Utilities|Casting|CastToBP_TaskSettings_ResurceDelivery Settings)
    (:then
      (CallFunction|InitializeTask (Variables|/Game/BoxStrategy/TaskSystem/Tasks/Settings/BP_TaskSettings_ResurceDelivery.BP_TaskSettings_ResurceDelivery_C|GetRequestedResources _asbp_task_settings_resurce_delivery)))
    (:CastFailed
      (CallFunction|BoxStrategyPrintStringError self "Event_InitializeTaskWithSettings" "Cannot cast to Task Settings" (Utilities|GetDisplayName Settings))
      (CallFunction|CloseThisTask))))

(event EventTryAssignUnitstoTask
  (params (UnitsToAssign :type Array%20of%20Object%20Object%20References))
  (for _array_element UnitsToAssign
    (bind _returnvalue (CallFunction|CanUnitWorkonThisTask _array_element))
    (if _returnvalue
      (Class|SearchingWorkObjectInterface|NewTaskAssigned(Message) _array_element self))))

(fn IsAvailableWorkPlace
  (if (|CallParentFunction)
    (bind _keys (Utilities|Map|Keys (Variables|Default|GetResources_Demand)))
    (for _array_element _keys
      (if (> (Public|ResourceAmountLeftforReserve _array_element) 0)
        (return true)))
    (return false)
    (else
      (return false))))

(fn WhatResorucesNeeded
  (if (Utilities|Enum|Equal(Enum) (Class|BoxStrategyUnitTask|GetTaskCurrentStatus) "Active")
    (bind _keys (Utilities|Map|Keys (Variables|Default|GetResources_Demand)))
    (for _array_element _keys
      (LocalVariables|SetLocal_SearchableResource _array_element)
      (LocalVariables|SetLocal_LeftAmount (Public|ResourceAmountLeftforReserve (LocalVariables|GetLocal_SearchableResource)))
      (if (> (LocalVariables|GetLocal_LeftAmount) 0)
        (Utilities|Map|Add (LocalVariables|GetLocal_ResourcesNeeded) (LocalVariables|GetLocal_SearchableResource) (LocalVariables|GetLocal_LeftAmount))))
    (return (LocalVariables|GetLocal_ResourcesNeeded))
    (else
      (CallFunction|BoxStrategyPrintStringError self "WhatResorucesNeeded" "Кто-то сделал запрос на количество необходимых ресурсов. Но состояние задачи не активно. Текущее состояние: " (Utilities|String|EnumtoString (Class|BoxStrategyUnitTask|GetTaskCurrentStatus)))
      (return 0))))

(fn ReserveResources
  (params (WhoReserves :type Object%20Object%20Reference) (WantReserveResources :type Map%20of%20Box%20Strategy%20Product%20Data%20Base%20Object%20References%20to%20Integers))
  (if (Utilities|Enum|Equal(Enum) (Class|BoxStrategyUnitTask|GetTaskCurrentStatus) "Active")
    (bind _keys (Utilities|Map|Keys WantReserveResources))
    (if (> (Utilities|Array|Length _keys) 0)
      (for _array_element _keys
        (LocalVariables|SetLocal_SearchableResource _array_element)
        (LocalVariables|SetLocal_AmountLeft (Public|ResourceAmountLeftforReserve (LocalVariables|GetLocal_SearchableResource)))
        (if (> (LocalVariables|GetLocal_AmountLeft) 0)
          (LocalVariables|SetLocal_WantReserveAmount (.Value (Utilities|Map|Find WantReserveResources (LocalVariables|GetLocal_SearchableResource))))
          (if (and (>= (LocalVariables|GetLocal_AmountLeft) (LocalVariables|GetLocal_WantReserveAmount)) (> (LocalVariables|GetLocal_WantReserveAmount) 0))
            (Utilities|Map|Add (LocalVariables|GetLocal_CanReserveThisResources) (LocalVariables|GetLocal_SearchableResource) (LocalVariables|GetLocal_WantReserveAmount))
            (Utilities|Map|Add (Variables|Default|GetResources_Reserved) (LocalVariables|GetLocal_SearchableResource) (+ (Public|GetReservedResourceAmount (LocalVariables|GetLocal_SearchableResource)) (LocalVariables|GetLocal_WantReserveAmount)))
            (LocalVariables|SetHaveReserved true :!label _label)
            (elif (> (LocalVariables|GetLocal_WantReserveAmount) 0)
              (|Error_ResourceAlreadyHave_2 (LocalVariables|GetLocal_SearchableResource))
              (Utilities|Map|Add (LocalVariables|GetLocal_CanReserveThisResources) (LocalVariables|GetLocal_SearchableResource) (LocalVariables|GetLocal_AmountLeft))
              (Utilities|Map|Add (Variables|Default|GetResources_Reserved) (LocalVariables|GetLocal_SearchableResource) (+ (Public|GetReservedResourceAmount) (LocalVariables|GetLocal_AmountLeft)))
              (goto _label)
              (else
                (|Error_ResourceAlreadyHave_2_2 (LocalVariables|GetLocal_SearchableResource)))))
          (else
            (|Error_ResourceAlreadyHave (LocalVariables|GetLocal_SearchableResource)))))
      (if (LocalVariables|GetHaveReserved)
        (Class|BoxStrategyUnitTask|AddNewWorker WhoReserves)
        (return (LocalVariables|GetLocal_CanReserveThisResources))
        (else
          (Development|PrintString (CallFunction|GetTaskOwnerActor) "No resources were reserved for task")
          (return (LocalVariables|GetLocal_CanReserveThisResources))))
      (else
        (Development|PrintString (CallFunction|GetTaskOwnerActor) (Utilities|String|Append "BP_Task_BringReources::ReserveResources(). TMap came empty from: " (Utilities|GetDisplayName WhoReserves)) true true "(R=1.000000,G=0.076040,B=0.000000,A=1.000000)" 1e+02)
        (return (LocalVariables|GetLocal_CanReserveThisResources))))
    (else
      (Development|PrintString (CallFunction|GetTaskOwnerActor) (Utilities|String|Append "BP_Task_BringResources::ReserveResources(). Task was finished but someone tries to reserve new deliver. Who: " (Utilities|GetDisplayName WhoReserves)))
      (return (LocalVariables|GetLocal_CanReserveThisResources)))))

(fn ResourceAmountLeftforReserve
  (params (Resource :type Box%20Strategy%20Product%20Data%20Base%20Object%20Reference%20%28by%20ref%29))
  (return (- (Public|GetBaseDemandResourceAmount Resource) (+ (Public|GetReservedResourceAmount Resource) (Public|GetDeliveredResourceAmount Resource)))))

(fn DeliverResources
  (params (DeliveredResources :type Map%20of%20Box%20Strategy%20Product%20Data%20Base%20Object%20References%20to%20Integers) (WhoDelivered :type Object%20Object%20Reference))
  (if (Utilities|Enum|Equal(Enum) (Class|BoxStrategyUnitTask|GetTaskCurrentStatus) "Active")
    (LocalVariables|SetLocal_DeliveredResources DeliveredResources)
    (bind _keys (Utilities|Map|Keys (LocalVariables|GetLocal_DeliveredResources)))
    (if (> (Utilities|Array|Length _keys) 0)
      (for _array_element _keys
        (LocalVariables|SetLocal_SearchableResource _array_element)
        (LocalVariables|SetLocal_DeliveredAmount (.Value (Utilities|Map|Find (LocalVariables|GetLocal_DeliveredResources) (LocalVariables|GetLocal_SearchableResource))))
        (if (>= (Public|GetReservedResourceAmount (LocalVariables|GetLocal_SearchableResource)) (LocalVariables|GetLocal_DeliveredAmount))
          _
          (else
            (|ErrorMessage_2)
            (LocalVariables|SetLocal_DeliveredAmount (Public|GetReservedResourceAmount (LocalVariables|GetLocal_SearchableResource)))))
        (Private|RemoveAmountfrom (Variables|Default|GetResources_Reserved) (LocalVariables|GetLocal_SearchableResource) (LocalVariables|GetLocal_DeliveredAmount))
        (private|AddAmountto (Variables|Default|GetResources_Delivered) (LocalVariables|GetLocal_SearchableResource) (LocalVariables|GetLocal_DeliveredAmount))
        (if (< (Public|ResourceAmountLeftforReserve (LocalVariables|GetLocal_SearchableResource)) 0)
          (CallFunction|BoxStrategyPrintStringError self "DeliverResources" "Кто-то принес ресурсов больше, чем нужно. Кто:" (Utilities|GetDisplayName WhoDelivered))))
      (else
        (CallFunction|BoxStrategyPrintStringError self "DeliverResources" "Кто-то принес пустой массив данных. Кто: " (Utilities|GetDisplayName WhoDelivered))))
    (Class|BoxStrategyUnitTask|RemoveWorker WhoDelivered)
    (Default|CallOnTaskWasUpdated)
    (if (CallFunction|IsAllResourcesDelivered)
      (CallFunction|CompleteTask))
    (return)
    (else
      (CallFunction|BoxStrategyPrintStringError self "DeliverResources" "Задача была выполнена, но кто-то попытался еще раз принести ресурс. Кто: " (Utilities|GetDisplayName WhoDelivered))
      (return))))

(fn AddAmountto
  (params (Map :type Map%20of%20Box%20Strategy%20Product%20Data%20Base%20Object%20References%20to%20Integers) (Resource :type Box%20Strategy%20Product%20Data%20Base%20Object%20Reference) (Amount :type Integer))
  (Utilities|Map|Add Map Resource (+ (.Value (Utilities|Map|Find Map Resource)) Amount)))

(fn RemoveAmountfrom
  (params (Map :type Map%20of%20Box%20Strategy%20Product%20Data%20Base%20Object%20References%20to%20Integers) (Resource :type Box%20Strategy%20Product%20Data%20Base%20Object%20Reference%20%28by%20ref%29) (Amount :type Integer))
  (Utilities|Map|Add Map Resource (- (.Value (Utilities|Map|Find Map Resource)) Amount)))

(fn GetTaskProgressPercent
  (return (Public|GetTaskPercent)))

(fn UnreserveResources
  (params (Resources_Reserved :type Map%20of%20Box%20Strategy%20Product%20Data%20Base%20Object%20References%20to%20Integers) (Who :type Object%20Object%20Reference))
  (bind _keys (Utilities|Map|Keys Resources_Reserved))
  (for _array_element _keys
    (if (>= (- (.Value (Utilities|Map|Find (Variables|Default|GetResources_Reserved) _array_element)) (.Value (Utilities|Map|Find Resources_Reserved _array_element))) 0)
      (Utilities|Map|Add (Variables|Default|GetResources_Reserved) _array_element (- (.Value (Utilities|Map|Find (Variables|Default|GetResources_Reserved) _array_element)) (.Value (Utilities|Map|Find Resources_Reserved _array_element))))
      (else
        (CallFunction|BoxStrategyPrintStringError self "UnreserveResources" "При попытке снять резерв сумма получилась отрицательной"))))
  (Class|BoxStrategyUnitTask|RemoveWorker Who)
  (return))

(fn GetReservedResourceAmount
  (params (Resource :type Box%20Strategy%20Product%20Data%20Base%20Object%20Reference%20%28by%20ref%29))
  (bind _resources_reserved (Variables|Default|GetResources_Reserved))
  (bind (_value _returnvalue) (Utilities|Map|Find _resources_reserved Resource))
  (if _returnvalue
    (return _value)
    (else
      (return 0))))

(fn GetBaseDemandResourceAmount
  (params (Resource :type Box%20Strategy%20Product%20Data%20Base%20Object%20Reference%20%28by%20ref%29))
  (bind _resources_demand (Variables|Default|GetResources_Demand))
  (bind (_value _returnvalue) (Utilities|Map|Find _resources_demand Resource))
  (if _returnvalue
    (return _value)
    (else
      (return 0))))

(fn GetTaskPercent
  (bind _keys (Utilities|Map|Keys (Variables|Default|GetResources_Demand)))
  (for _array_element _keys
    (LocalVariables|SetLocal_DemandAmount (+ (LocalVariables|GetLocal_DemandAmount) (.Value (Utilities|Map|Find (Variables|Default|GetResources_Demand) _array_element))))
    (LocalVariables|SetLocal_DeliveredAmount (+ (LocalVariables|GetLocal_DeliveredAmount) (.Value (Utilities|Map|Find (Variables|Default|GetResources_Delivered) _array_element)))))
  (return (/ (Math|Conversions|ToFloat(Integer) (LocalVariables|GetLocal_DeliveredAmount)) (Math|Conversions|ToFloat(Integer) (LocalVariables|GetLocal_DemandAmount)))))

(fn GetDeliveredResourceAmount
  (params (Resource :type Box%20Strategy%20Product%20Data%20Base%20Object%20Reference%20%28by%20ref%29))
  (bind _resources_delivered (Variables|Default|GetResources_Delivered))
  (bind (_value _returnvalue) (Utilities|Map|Find _resources_delivered Resource))
  (if _returnvalue
    (return _value)
    (else
      (return 0))))

(fn CloseThisTask
  (|CallParentFunction)
  (if (Utilities|Enum|NotEqual(Enum) (Class|BoxStrategyUnitTask|GetTaskCurrentStatus) "Canceled")
    _
    (else
      (CallFunction|BoxStrategyPrintStringError self "CloseThisTask" "Таска закрывается, но она не завершена. Здесь должен быть спаун ресурсов, которые были занесены в таску на место здания. Текущее состояние: " (Utilities|String|EnumtoString (Class|BoxStrategyUnitTask|GetTaskCurrentStatus)))))
  (return))

(fn IsAllResourcesDelivered
  (bind _keys (Utilities|Map|Keys (Variables|Default|GetResources_Delivered)))
  (for _array_element _keys
    (if (!= (.Value (Utilities|Map|Find (Variables|Default|GetResources_Delivered) _array_element)) (.Value (Utilities|Map|Find (Variables|Default|GetResources_Demand) _array_element)))
      (return false)))
  (return true))

(fn InitializeTask
  (params (Resources_Demand :type Map%20of%20Box%20Strategy%20Product%20Data%20Base%20Object%20References%20to%20Integers))
  (Variables|Default|SetResources_Demand Resources_Demand)
  (Utilities|Map|Clear (Variables|Default|GetResources_Reserved))
  (Utilities|Map|Clear (Variables|Default|GetResources_Delivered))
  (bind _keys (Utilities|Map|Keys (Variables|Default|GetResources_Demand)))
  (if (> (Utilities|Array|Length _keys) 0)
    (for _array_element _keys
      (Utilities|Map|Add (Variables|Default|GetResources_Reserved) _array_element 0)
      (Utilities|Map|Add (Variables|Default|GetResources_Delivered) _array_element 0))
    (Default|CallOnTaskInitializationFinished)
    (else
      (CallFunction|BoxStrategyPrintStringError self "Event_InitializeTask" "Resources Demand is Empty. Task cannot work.")
      (CallFunction|CloseThisTask))))

(fn CanUnitWorkonThisTask
  (params (TaskSearchingUnit :type Object%20Object%20Reference))
  (return (CallFunction|IsAvailableWorkPlace)))