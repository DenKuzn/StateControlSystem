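; Base task Blueprint for the BoxStrategy task system, supplying status, worker-slot and lifecycle logic, with empty initialization events and a zero default progress.
; The task's outer object serves as its owner actor and supplies its location.
; Work places are available only while the task is Active and below its worker limit.
; Completing sets Completed and broadcasts finished; closing clears workers, cancels a still-Active task, then broadcasts closed.
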(event Custom|SimpleInitializeTask)

(event Custom|InitializeTaskWithSettings
  (params (Settings :type BP%20Task%20Settings%20Base%20Object%20Reference)))

(fn IsAvailableWorkPlace
  (return (and (Utilities|Enum|Equal(Enum) (Class|BoxStrategyUnitTask|GetTaskCurrentStatus) "Active") (< (Class|BoxStrategyUnitTask|GetCurrentWorkersNum) (Class|BoxStrategyUnitTask|GetMaxWorkers)))))

(fn GetTaskOwnerActor
  (return (.AsActor (Utilities|Casting|CastToActor (Utilities|GetOuterObject self)))))

(fn CloseThisTask
  (Class|BoxStrategyUnitTask|ClearAllWorkers)
  (switch Utilities|FlowControl|Switch|SwitchonEBoxStrategyUnitTaskState (Class|BoxStrategyUnitTask|GetTaskCurrentStatus)
    (:Active
      (Class|BoxStrategyUnitTask|SetTaskCurrentStatus "Canceled")
      (Default|CallOnTaskWasCanceled))
    (:Completed
      _)
    (:Canceled
      _))
  (Default|CallOnTaskWasClosed self)
  (return))

(fn GetTaskLocation
  (return (Transformation|GetActorLocation (Public|GetTaskOwnerActor))))

(fn GetTaskProgressPercent
  (return 0.0))

(fn CompleteTask
  (Class|BoxStrategyUnitTask|SetTaskCurrentStatus "Completed")
  (Default|CallOnTaskWasFinished)
  (return))