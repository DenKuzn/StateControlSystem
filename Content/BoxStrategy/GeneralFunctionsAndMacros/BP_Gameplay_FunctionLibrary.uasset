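; Gameplay function library for Box Strategy, holding small shared helpers for error reporting, grid math and robot tasks.
; The error helper prints a long-lasting red on-screen message naming the failing function.
; Grid recalculation snaps a vector per axis to GridSize multiples by integer conversion rather than explicit rounding.
; A tag bridge switches robot task tags (resource delivery, building construction) to their matching ability tags.
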(fn BoxStrategyPrintStringError
  (params (Object :type Object%20Object%20Reference) (Function%20Name :type String) (MessageText :type String) (AdditionalInformation :type String))
  (Development|PrintString Object (Utilities|String|Append "Error: " Function%20Name "(). " MessageText " / " AdditionalInformation) true true "(R=1.000000,G=0.000000,B=0.000000,A=1.000000)" 1e+02))

(fn RecalculatetoGridPosition
  (params (InVec :type Vector) (GridSize :type Float%20%28double-precision%29))
  (bind (_x _y _z) (Math|Vector|BreakVector InVec))
  (return (Math|Vector|MakeVector (Math|Conversions|ToFloat(Integer) (* (Class|KismetMathLibrary|ToInt64(Float) (/ _x GridSize)) GridSize)) (Math|Conversions|ToFloat(Integer) (* (Class|KismetMathLibrary|ToInt64(Float) (/ _y GridSize)) GridSize)) (Math|Conversions|ToFloat(Integer) (* (Class|KismetMathLibrary|ToInt64(Float) (/ _z GridSize)) GridSize)))))

(fn GetAbilityTagfromTaskTagRobotsBridge
  (params (TaskTag :type Gameplay%20Tag%20Structure))
  (|SwitchGameplayTag TaskTag
    (:Default
      (return "(TagName=\"\")"))
    (:BoxStrategy.Tasks.RobotTasks.ResourceDelivery
      (return "(TagName=\"BoxStrategy.SelectableObjects.Robots.Abilities.ResourceDelivery\")"))
    (:BoxStrategy.Tasks.RobotTasks.ConstructBuilding
      (return "(TagName=\"BoxStrategy.SelectableObjects.Robots.Abilities.ConstructBuilding\")"))))