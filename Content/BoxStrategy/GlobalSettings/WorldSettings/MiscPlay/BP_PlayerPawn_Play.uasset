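; Player pawn for strategy play that serves as a top-level camera rig driven by Enhanced Input, adding the base mapping context for the local player.
; Input pans the pawn locally and yaws it, with pan speed scaling with zoom distance.
; Scroll sets a clamped spring arm target length, which Tick interpolates toward on the locally controlled pawn.
; Action and back button events are empty, as a note assigns input handling to State Controls.
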(event Input|EnhancedActionEvents|EnhancedInputActionIA_CameraScroll
  (params (ActionValue :type Float%20%28double-precision%29) (ElapsedSeconds :type Float%20%28double-precision%29) (TriggeredSeconds :type Float%20%28double-precision%29) (InputAction :type Input%20Action%20Object%20Reference :default "/Game/BoxStrategy/GlobalSettings/WorldSettings/MiscPlay/BaseInputs/Actions/IA_CameraScroll.IA_CameraScroll"))
  ;[0.1045 0.01591 0.1997] Main Camera Control
  (Variables|Camera|SpringArm|SetSpringArm_NewLengthTarget (Math|Float|Clamp(Float) (+ (* (Variables|Camera|SpringArm|GetSpringArm_CameraZoomStep) ActionValue) (Variables|Camera|SpringArm|GetSpringArm_NewLengthTarget)) (Variables|Camera|SpringArm|GetSpringArm_Min) (Variables|Camera|SpringArm|GetSpringArm_Max))))

(event Input|EnhancedActionEvents|EnhancedInputActionIA_CameraMovement
  (params (ActionValue :type Vector%202D%20Structure) (ElapsedSeconds :type Float%20%28double-precision%29) (TriggeredSeconds :type Float%20%28double-precision%29) (InputAction :type Input%20Action%20Object%20Reference :default "/Game/BoxStrategy/GlobalSettings/WorldSettings/MiscPlay/BaseInputs/Actions/IA_CameraMovement.IA_CameraMovement"))
  (bind _returnvalue (CallFunction|CalculateCameraMovementMultiplier))
  (bind _returnvalue_2 (Math|Vector2D|Normalize2D ActionValue))
  (bind _returnvalue_3 (* _returnvalue_2 _returnvalue))
  ;[0.1045 0.01591 0.1997] Main Camera Control
  (Transformation|AddActorLocalOffset (Math|Vector|MakeVector (.x _returnvalue_3) (.y _returnvalue_3) 0.0) false false))

(event Input|EnhancedActionEvents|EnhancedInputActionIA_ActionButton
  (params (ActionValue :type Boolean) (ElapsedSeconds :type Float%20%28double-precision%29) (TriggeredSeconds :type Float%20%28double-precision%29) (InputAction :type Input%20Action%20Object%20Reference :default "/Game/BoxStrategy/GlobalSettings/WorldSettings/MiscPlay/BaseInputs/Actions/IA_ActionButton.IA_ActionButton"))
  ;[1 0 0.3375] State Controls должны самостоятельно полностью обрабатывать инпуты игрока, чтобы контролировать состояние игры на самом высоком уровне.
  ; Для этого в классе State Controls есть функция StateControlInputTriggered, которая возвращает InputTag (тег инпута) и bool - нажато или отжато.
)

(event Input|EnhancedActionEvents|EnhancedInputActionIA_BackButton
  (params (ActionValue :type Boolean) (ElapsedSeconds :type Float%20%28double-precision%29) (TriggeredSeconds :type Float%20%28double-precision%29) (InputAction :type Input%20Action%20Object%20Reference :default "/Game/BoxStrategy/GlobalSettings/WorldSettings/MiscPlay/BaseInputs/Actions/IA_BackButton.IA_BackButton"))
  ;[1 0 0.3375] State Controls должны самостоятельно полностью обрабатывать инпуты игрока, чтобы контролировать состояние игры на самом высоком уровне.
  ; Для этого в классе State Controls есть функция StateControlInputTriggered, которая возвращает InputTag (тег инпута) и bool - нажато или отжато.
)

(event Input|EnhancedActionEvents|EnhancedInputActionIA_CameraRotation
  (params (ActionValue :type Float%20%28double-precision%29) (ElapsedSeconds :type Float%20%28double-precision%29) (TriggeredSeconds :type Float%20%28double-precision%29) (InputAction :type Input%20Action%20Object%20Reference :default "/Game/BoxStrategy/GlobalSettings/WorldSettings/MiscPlay/BaseInputs/Actions/IA_CameraRotation.IA_CameraRotation"))
  (Class|Actor|AddActorWorldRotation (Math|Rotator|MakeRotator 0.0 0.0 (* ActionValue (Variables|Camera|Movement|GetCameraRotation_Angle)))))

(event EventBeginPlay
  (if (Pawn|IsLocallyControlled)
    (Variables|Camera|SpringArm|SetSpringArm_NewLengthTarget (Variables|/Script/Engine.SpringArmComponent|GetTargetArmLength (Variables|Default|GetSpringArm)))
    (Input|AddMappingContext (PlayerController|LocalPlayerSubsystems|GetEnhancedInputLocalPlayerSubsystem (Game|GetPlayerController 0)) "/Game/BoxStrategy/GlobalSettings/WorldSettings/MiscPlay/BaseInputs/Contexts/IMC_BaseInputs.IMC_BaseInputs" 0 "(bIgnoreAllPressedKeysUntilRelease=True,bForceImmediately=False,bNotifyUserSettings=False)")))

(event EventTick
  (params (DeltaSeconds :type Float%20%28single-precision%29))
  (if (Pawn|IsLocallyControlled)
    (CallFunction|InterpSpringArmLenghttoTarget 5.0)))

(event Input|KeyboardEvents|F
  (params (Key :type Key%20Structure :default "None")))

(fn ConstructionScript)

(fn InterpSpringArmLenghttoTarget
  (params (InterSpeed :type Float%20%28double-precision%29))
  (if (not (Math|Float|NearlyEqual(Float) (Variables|/Script/Engine.SpringArmComponent|GetTargetArmLength (Variables|Default|GetSpringArm)) (Variables|Camera|SpringArm|GetSpringArm_NewLengthTarget) 0.0001))
    (Variables|/Script/Engine.SpringArmComponent|SetTargetArmLength (Variables|Default|GetSpringArm) (Math|Interpolation|FInterpTo (Variables|/Script/Engine.SpringArmComponent|GetTargetArmLength (Variables|Default|GetSpringArm)) (Variables|Camera|SpringArm|GetSpringArm_NewLengthTarget) (Utilities|Time|GetWorldDeltaSeconds) InterSpeed))))

(fn CalculateCameraMovementMultiplier
  (return (+ (Variables|Camera|Movement|GetCameraMovement_SpeedMultiplier) (* (/ (- (Variables|Camera|SpringArm|GetSpringArm_NewLengthTarget) (Variables|Camera|SpringArm|GetSpringArm_Min)) (- (Variables|Camera|SpringArm|GetSpringArm_Max) (Variables|Camera|SpringArm|GetSpringArm_Min))) (Variables|Camera|Movement|GetCameraMovement_AltitudeSpeedMultiplier)))))

(fn RotateCameraDetection)

(fn MoveCameraDetection)