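; Production stage that handles constructing a building by delegating the work to a construction task.
; On activation it creates the task with the stage's production points as the requested amount and registers it with the player state's task manager component.
; Task updates propagate as stage updates, finishing closes the task and completes the stage, and cancelling closes it.
; Stage progress mirrors the task's progress percent, logging an error when the task is invalid.
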(event Custom|Event_TaskWasUpdated
  (Default|CallOnStageUpdated self))

(event Custom|Event_TaskWasFinished
  (Default|CloseThisTask (Variables|Default|GetConstructionTask))
  (Class|ProductionStageBase|CurrentStageCompleted)
  (Variables|Default|SetConstructionTask 0))

(event EventActivateExecution
  (bind _returnvalue (Game|ConstructObjectfromClass (Class|ProductionStageBase|GetOwnerActor) "/Game/BoxStrategy/TaskSystem/Tasks/BP_Task_ConstructBuilding.BP_Task_ConstructBuilding_C"))
  (Variables|Default|SetConstructionTask _returnvalue)
  (EventDispatchers|BindEventtoOnTaskWasUpdated (Variables|Default|GetConstructionTask) (EventDispatchers|CreateEvent :!event Custom|Event_TaskWasUpdated))
  (EventDispatchers|BindEventtoOnTaskWasFinished (Variables|Default|GetConstructionTask) (EventDispatchers|CreateEvent :!event Custom|Event_TaskWasFinished))
  (bind _returnvalue_2 (Game|ConstructObjectfromClass (Variables|Default|GetConstructionTask) "/Game/BoxStrategy/TaskSystem/Tasks/Settings/BP_TaskSettings_ConstructBuilding.BP_TaskSettings_ConstructBuilding_C" (Variables|/Script/BoxStrategy.BoxStrategyProductData_Base|GetProductionPoints (Class|ProductionStageBase|GetProductionData))))
  (Default|InitializeTaskwithSettings (Variables|Default|GetConstructionTask) _returnvalue_2)
  (Default|EventAddNewTask (Actor|GetComponentbyClass (Game|GetPlayerState 0) "/Game/BoxStrategy/TaskSystem/BaseSystem/BP_TaskManagerComponent.BP_TaskManagerComponent_C") (Variables|Default|GetConstructionTask)))

(event EventCancelExecution
  (Default|CloseThisTask (Variables|Default|GetConstructionTask))
  (Variables|Default|SetConstructionTask 0))

(fn GetStageProgress
  (Utilities|IsValid (Variables|Default|GetConstructionTask)
    (:Is%20Valid
      (return (Default|GetTaskProgressPercent (Variables|Default|GetConstructionTask))))
    (:Is%20Not%20Valid
      (CallFunction|BoxStrategyPrintStringError self "GetStageProgress" "Task Invalid")
      (return 0.0))))