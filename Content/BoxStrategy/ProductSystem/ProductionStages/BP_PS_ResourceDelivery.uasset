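; BP_PS_ResourceDelivery is a production stage that completes once the resources requested by its production data are delivered through a task.
; On activation it constructs a delivery task with those resources as settings and registers it with the task manager on the player state.
; Task updates are relayed as stage updates and supply the progress percentage.
; Finishing closes the task and completes the stage, while cancelling only closes it.
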(event Custom|Event_TaskWasUpdated
  (Default|CallOnStageUpdated self))

(event Custom|Event_TaskWasFinished
  (Default|CloseThisTask (Variables|Default|GetDeliveryTask))
  (Class|ProductionStageBase|CurrentStageCompleted)
  (Variables|Default|SetDeliveryTask 0))

(event EventActivateExecution
  (bind _returnvalue (Game|ConstructObjectfromClass (Class|ProductionStageBase|GetOwnerActor) "/Game/BoxStrategy/TaskSystem/Tasks/BP_Task_ResourceDelivery.BP_Task_ResourceDelivery_C"))
  (Variables|Default|SetDeliveryTask _returnvalue)
  (EventDispatchers|BindEventtoOnTaskWasUpdated (Variables|Default|GetDeliveryTask) (EventDispatchers|CreateEvent :!event Custom|Event_TaskWasUpdated))
  (EventDispatchers|BindEventtoOnTaskWasFinished (Variables|Default|GetDeliveryTask) (EventDispatchers|CreateEvent :!event Custom|Event_TaskWasFinished))
  (bind _returnvalue_2 (Game|ConstructObjectfromClass (Variables|Default|GetDeliveryTask) "/Game/BoxStrategy/TaskSystem/Tasks/Settings/BP_TaskSettings_ResurceDelivery.BP_TaskSettings_ResurceDelivery_C" (Variables|/Script/BoxStrategy.BoxStrategyProductData_Base|GetRequestedObjects (Class|ProductionStageBase|GetProductionData))))
  (Default|InitializeTaskwithSettings (Variables|Default|GetDeliveryTask) _returnvalue_2)
  (Default|EventAddNewTask (Actor|GetComponentbyClass (Game|GetPlayerState 0) "/Game/BoxStrategy/TaskSystem/BaseSystem/BP_TaskManagerComponent.BP_TaskManagerComponent_C") (Variables|Default|GetDeliveryTask)))

(event EventCancelExecution
  (Default|CloseThisTask (Variables|Default|GetDeliveryTask))
  (Variables|Default|SetDeliveryTask 0))

(fn GetStageProgress
  (Utilities|IsValid (Variables|Default|GetDeliveryTask)
    (:Is%20Valid
      (return (Default|GetTaskProgressPercent (Variables|Default|GetDeliveryTask))))
    (:Is%20Not%20Valid
      (CallFunction|BoxStrategyPrintStringError self "GetStageProgress" "Task Invalid")
      (return 0.0))))