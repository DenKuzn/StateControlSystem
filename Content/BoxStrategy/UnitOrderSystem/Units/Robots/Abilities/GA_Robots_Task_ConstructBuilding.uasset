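; Gameplay ability that sends a robot to carry out a construct-building task in the unit order system.
; It takes the task from its ability settings and moves the avatar by AI until it overlaps the task owner.
; A re-armed one-second timer then adds production points while the task stays active.
; Task closure or an invalid task triggers a randomly delayed end, and ending clears timers, bindings and movement.
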(event Custom|Event_AvatarOverlappedSomething
  (params (OverlappedActor :type Actor%20Object%20Reference) (OtherActor :type Actor%20Object%20Reference))
  (bind _returnvalue (Ability|GetAvatarActorfromActorInfo))
  (Utilities|IsValid (Variables|Default|GetMyTask)
    (:Is%20Valid
      (if (== (Default|GetTaskOwnerActor (Variables|Default|GetMyTask)) OtherActor)
        (Collision|UnbindEventfromOnActorBeginOverlap _returnvalue (EventDispatchers|CreateEvent :!event Custom|Event_AvatarOverlappedSomething))
        (AI|Navigation|StopMovement (AI|GetAIController _returnvalue))
        (CallFunction|EventStartGatherProductionPoint)))
    (:Is%20Not%20Valid
      (CallFunction|BoxStrategyPrintStringError self "Event_AvatarOverlappedSomething" "MyTask invalid")
      (CallFunction|EventEndAbilitywithDelay))))

(event Custom|Event_EndAbilityWithDelay
  ;[1 0 0] TODO:
  ; - Таймер понадобился второй раз. А значит, это нужно вынести в базовый класс.
  ; Добавить так же снос таймера на завершении абилки.
  (if (not (Utilities|Time|IsTimerActivebyHandle (Variables|Default|GetTimer_EndAbility)))
    (bind _returnvalue (Utilities|Time|SetTimerbyEvent (EventDispatchers|CreateEvent :!event K2EndAbility) (Math|Random|RandomFloatinRange 0.04 1.0)))
    (Variables|Default|SetTimer_EndAbility _returnvalue)
    (else
      (CallFunction|BoxStrategyPrintStringError self "Event_TryGetNewResource" "Ресурсы не найдены для доставки, поэтому сброс абилки. Но таймер уже активен."))))

(event Custom|Event_TaskWasClosed
  (params (Task :type BP%20Task%20Base%20Object%20Reference))
  (CallFunction|EventEndAbilitywithDelay))

(event Custom|Event_AddNewProductPointToTask
  (Utilities|IsValid (Variables|Default|GetMyTask)
    (:Is%20Valid
      (if (Utilities|Enum|Equal(Enum) (Class|BoxStrategyUnitTask|GetTaskCurrentStatus (Variables|Default|GetMyTask)) "Active")
        (Default|EventAddProductionPoint (Variables|Default|GetMyTask) 1.0)
        (if (Utilities|Enum|Equal(Enum) (Class|BoxStrategyUnitTask|GetTaskCurrentStatus (Variables|Default|GetMyTask)) "Active")
          (CallFunction|EventStartGatherProductionPoint)
          (else
            (Ability|EndAbility :!label _label)))
        (else
          (goto _label))))
    (:Is%20Not%20Valid
      (goto _label))))

(event Custom|Event_StartGatherProductionPoint
  (Development|PrintString "Started producting points")
  (Utilities|IsValid (Variables|Default|GetMyTask)
    (:Is%20Valid
      (bind _returnvalue (Utilities|Time|SetTimerbyEvent (delegate Custom|Event_AddNewProductPointToTask) 1.0))
      (Variables|Default|SetTimer_ProdductionPoint _returnvalue))
    (:Is%20Not%20Valid
      (CallFunction|BoxStrategyPrintStringError self "Event_StartAddProductionPoints" "MyTask invalid")
      (CallFunction|EventEndAbilitywithDelay))))

(event Ability|EventActivateAbility
  (CallFunction|GetMyTask)
  (Utilities|IsValid (Variables|Default|GetMyTask)
    (:Is%20Valid
      (EventDispatchers|BindEventtoOnTaskWasClosed (Variables|Default|GetMyTask) (delegate Custom|Event_TaskWasClosed))
      (if (not (Collision|IsOverlappingActor (Ability|GetAvatarActorfromActorInfo) (Default|GetTaskOwnerActor (Variables|Default|GetMyTask)) :!class /Script/Engine.Actor))
        (Collision|BindEventtoOnActorBeginOverlap (Ability|GetAvatarActorfromActorInfo) (EventDispatchers|CreateEvent :!event Custom|Event_AvatarOverlappedSomething))
        (AI|AIMoveTo (.AsPawn (Utilities|Casting|CastToPawn (Ability|GetAvatarActorfromActorInfo))) (Default|GetTaskLocation (Variables|Default|GetMyTask)) 0 5.0 false)
        (else
          (CallFunction|EventStartGatherProductionPoint))))
    (:Is%20Not%20Valid
      (CallFunction|BoxStrategyPrintStringError self "ActivateAbility" "MyTask invalid")
      (CallFunction|EventEndAbilitywithDelay))))

(event Ability|EventOnEndAbility
  (params (bWasCancelled :type Boolean))
  (CallFunction|ResetAbilityData)
  (Development|PrintString "Ability Ended"))

(fn GetMyTask
  (bind _asbp_task_construct_building (Utilities|Casting|CastToBP_Task_ConstructBuilding (Variables|/Game/BoxStrategy/UnitOrderSystem/Units/Robots/Settings/BP_UOAS_TaskReceiver.BP_UOAS_TaskReceiver_C|GetTaskToReceive (.AsBP%20UOAS%20Task%20Receiver (Utilities|Casting|CastToBP_UOAS_TaskReceiver (Class|UnitOrderGameplayAbility|GetMyAbilitySettings))))))
  (Variables|Default|SetMyTask _asbp_task_construct_building))

(fn ResetAbilityData
  (bind _returnvalue (Ability|GetAvatarActorfromActorInfo))
  (bind _returnvalue_2 (AI|GetAIController _returnvalue))
  (Utilities|FlowControl|Sequence
    (:then_0
      (Utilities|Time|ClearandInvalidateTimerbyHandle (Variables|Default|GetTimer_EndAbility))
      (Utilities|Time|ClearandInvalidateTimerbyHandle (Variables|Default|GetTimer_ProdductionPoint)))
    (:then_1
      ;[1 1 1] TODO: используется код второй раз (1 ResourceDelivery). Нужно вынести в базовый класс.
      (Utilities|IsValid (Ability|GetAvatarActorfromActorInfo)
        (:Is%20Valid
          (Collision|UnbindEventfromOnActorBeginOverlap _returnvalue (EventDispatchers|CreateEvent :!event Custom|Event_AvatarOverlappedSomething))
          (Utilities|IsValid _returnvalue_2
            (:Is%20Valid
              (AI|Navigation|StopMovement _returnvalue_2))))))
    (:then_2
      (Utilities|IsValid (Variables|Default|GetMyTask)
        (:Is%20Valid
          (EventDispatchers|UnbindEventfromOnTaskWasClosed (Variables|Default|GetMyTask) (EventDispatchers|CreateEvent :!event Custom|Event_TaskWasClosed)))))))