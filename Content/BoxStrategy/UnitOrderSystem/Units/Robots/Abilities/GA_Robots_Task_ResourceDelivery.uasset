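; Gameplay ability that makes a robot unit fulfil a resource delivery task by hauling ground items to the task's actor.
; It sphere-traces around the task for needed items, reserves amounts on item and task, walks over, takes them and delivers on overlap, showing a carried mesh en route.
; A destroyed item restarts the search, a failed search ends the ability after a random delay, and task cancellation drops carried resources on a grid-snapped spot.
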(event Custom|Event_ResourceWasDestroyed
  (params (DestroyedActor :type Actor%20Object%20Reference))
  ;[1 0.7141 0 0.217] Try To Get Resource Amount From Resource.
  ;;[0.1968 0.225 0.6677 0.108] Обработчики разилчных игровых ситуаций.
  (Variables|Reserved|SetReservedAmount 0)
  (Variables|Reserved|SetReservedResourceOnGround 0)
  (CallFunction|EventTryGetNewResource))

(event Custom|Event_TryGetNewResource
  ;[1 0.7141 0 0.217] Try To Get Resource Amount From Resource.
  (Utilities|IsValid (Variables|AbilitySettings|GetMyTask)
    (:Is%20Valid
      ;;[1 1 0 0.408] Резервация ресурса.
      (bind _findresources (CallFunction|FindandReserveResources))
      (if _findresources
        (if (not (CallFunction|IsResourceNear))
          ;;[1 0.7138 0 0.296] Движение за ресурсом.
          (Game|BindEventtoOnDestroyed (Variables|Reserved|GetReservedResourceOnGround) (EventDispatchers|CreateEvent :!event Custom|Event_ResourceWasDestroyed))
          (AI|AIMoveTo (.AsPawn (Utilities|Casting|CastToPawn (Ability|GetAvatarActorfromActorInfo))) (Transformation|GetActorLocation (Variables|Reserved|GetReservedResourceOnGround)) 0 (Variables|AbilitySettings|GetAcceptableRadius) false
            (:OnSuccess
              (Utilities|IsValid (Variables|Reserved|GetReservedResourceOnGround)
                (:Is%20Valid
                  (if (CallFunction|IsResourceNear)
                    (CallFunction|EventTakeResourceandTryDelivery)
                    (else
                      ;;[0.5844 0.07731 0.07731 0.304 12] Обработка ошибок
                      (CallFunction|BoxStrategyPrintStringError self "AI Move To" "Перс дошел, но ресур далеко.")
                      (CallFunction|EventResourceWasDestroyed :!label _label) ; Будем считать, что ресурс был уничтожен.
                    )))
                (:Is%20Not%20Valid
                  (CallFunction|BoxStrategyPrintStringError self "AI Move To" "ресурс сдох")
                  (goto _label)))))
          (else
            (CallFunction|EventTakeResourceandTryDelivery)))
        (else
          (CallFunction|EventEndAbilitywithDelay))))))

(event Custom|Event_TryDeliveryResourcesToTask
  (|CheckStatuses
    (:Is%20Valid
      ;[1 1 1 1 12] Ситуация, когда мы очень близко к зданию и уже находимсмся в момент подбора ресурса в зоне здания, чтобы принести ему ресурс.
      (if (not (CallFunction|IsUnitOverlappingTaskActor))
        (Collision|BindEventtoOnActorBeginOverlap (.AsCharacter (Utilities|Casting|CastToCharacter (Ability|GetAvatarActorfromActorInfo))) (EventDispatchers|CreateEvent :!event Custom|Event_CharacterOverlapSomething))
        (CallFunction|AddMeshtoCharacter)
        (AI|AIMoveTo (.AsPawn (Utilities|Casting|CastToPawn (Ability|GetAvatarActorfromActorInfo))) (Default|GetTaskLocation (Variables|AbilitySettings|GetMyTask)) 0 5.0 false)
        (else
          (CallFunction|DeliverResourcestoTaskandEndAbility))))))

(event Custom|Event_CharacterOverlapSomething
  (params (OverlappedActor :type Actor%20Object%20Reference) (OtherActor :type Actor%20Object%20Reference))
  (Utilities|IsValid (Variables|AbilitySettings|GetMyTask)
    (:Is%20Valid
      (if (== OtherActor (Default|GetTaskOwnerActor (Variables|AbilitySettings|GetMyTask)))
        (CallFunction|DeliverResourcestoTaskandEndAbility)))
    (:Is%20Not%20Valid
      (CallFunction|RespawnResourceNearRobot)
      (Ability|EndAbility))))

(event Custom|Event_TakeResourceAndTryDelivery
  ;[1 0.7141 0 0.217] Try To Get Resource Amount From Resource.
  ;;[0.1968 0.225 0.6677 0.108] Обработчики разилчных игровых ситуаций.
  (CallFunction|TakeResourcefromItemonGround)
  (CallFunction|EventTryDeliveryResourcestoTask))

(event Custom|Event_EndAbilityWithDelay
  ;[1 0.7141 0 0.217] Try To Get Resource Amount From Resource.
  ;;[0.1968 0.225 0.6677 0.108] Обработчики разилчных игровых ситуаций.
  (if (not (Utilities|Time|IsTimerActivebyHandle (Variables|Default|GetEndingTimer)))
    (bind _returnvalue (Utilities|Time|SetTimerbyEvent (EventDispatchers|CreateEvent :!event K2EndAbility) (Math|Random|RandomFloatinRange 0.04 1.0)))
    (Variables|Default|SetEndingTimer _returnvalue)
    (else
      (CallFunction|BoxStrategyPrintStringError self "Event_TryGetNewResource" "Ресурсы не найдены для доставки, поэтому сброс абилки. Но таймер уже активен."))))

(event Custom|Event_TaskWasCanceled
  (CallFunction|RespawnResourceNearRobot)
  (Ability|EndAbility))

(event Ability|EventActivateAbility
  (Utilities|CheckandSaveTask
    (:Is%20Valid
      (EventDispatchers|AssignOnTaskWasCanceled (Variables|AbilitySettings|GetMyTask) (delegate Custom|Event_TaskWasCanceled))
      (CallFunction|EventTryGetNewResource))))

(event Ability|EventOnEndAbility
  (params (bWasCancelled :type Boolean))
  (CallFunction|ResetAllData))

(fn FindandReserveResources
  (bind _mytask (Variables|AbilitySettings|GetMyTask))
  (bind _tasklocation (Default|GetTaskLocation _mytask))
  (if (Default|IsAvailableWorkPlace (Variables|AbilitySettings|GetMyTask))
    (bind _resourcesneeded (Default|WhatResorucesNeeded (Variables|AbilitySettings|GetMyTask)))
    (LocalVariables|SetLocal_NeededResources _resourcesneeded)
    (bind _keys (Utilities|Map|Keys (LocalVariables|GetLocal_NeededResources)))
    (bind _output_get (LocalVariables|SetLocal_NeededResourceDataAssets _keys))
    (if (> (Utilities|Array|Length _output_get) 0)
      (bind (_outhits _returnvalue) (Collision|MultiSphereTraceForObjects _tasklocation _tasklocation (Variables|AbilitySettings|GetSearchingRadius) (Utilities|Array|MakeArray "ObjectTypeQuery7") false 0 "ForDuration"))
      (if _returnvalue
        (for _array_element _outhits
          (bind _asbp_pickable_item_base (Utilities|Casting|CastToBP_PickableItem_Base (.HitActor (Collision|BreakHitResult _array_element))))
          (LocalVariables|SetLocal_FreeResourceOnGround _asbp_pickable_item_base)
          (for _array_element_2 (LocalVariables|GetLocal_NeededResourceDataAssets)
            (if (== (Default|GetItemType (LocalVariables|GetLocal_FreeResourceOnGround)) (Variables|/Script/BoxStrategy.BoxStrategyProductData_Base|GetMainTypeTag _array_element_2))
              (bind _aspickable_item_data_base (Utilities|Casting|CastToPickableItemData_Base _array_element_2))
              (bind (_can _availableamount) (Default|CanReservewithValidation (LocalVariables|GetLocal_FreeResourceOnGround)))
              (if _can
                (bind _amountreserved (Default|ReserveItemAmount (LocalVariables|GetLocal_FreeResourceOnGround) (Ability|GetAvatarActorfromActorInfo) (Math|Integer|Clamp(Integer) (Math|Integer|Clamp(Integer) _availableamount 0 (Variables|/Script/BoxStrategy.PickableItemData_Base|GetMaxStock _aspickable_item_data_base)) 0 (.Value (Utilities|Map|Find (LocalVariables|GetLocal_NeededResources) _aspickable_item_data_base)))))
                (CallFunction|SaveReservedData (LocalVariables|GetLocal_FreeResourceOnGround) _amountreserved _aspickable_item_data_base)
                (bind _reservedresources (Default|ReserveResources (Variables|AbilitySettings|GetMyTask) (Ability|GetAvatarActorfromActorInfo) (Utilities|Map|MakeMap (Variables|Reserved|GetReservedResourceData) (Variables|Reserved|GetReservedAmount))))
                (if (.ReturnValue (Utilities|Map|Find _reservedresources (Variables|Reserved|GetReservedResourceData)))
                  (if (== (.Value (Utilities|Map|Find _reservedresources (Variables|Reserved|GetReservedResourceData))) (Variables|Reserved|GetReservedAmount))
                    (return true)
                    (else
                      _)))
                (CallFunction|BoxStrategyPrintStringError self "FindAndreserveResources" "После того, как проверил необходимость ресурсов, нашел свободные ресурсы и зарезервировал для себя место в Таске - обнаружилось, что что-то не так, и резерв выдан либо не на нужный ресурс, либо другое количество.")
                (Default|UnreserveResources (Variables|AbilitySettings|GetMyTask) _reservedresources (Ability|GetAvatarActorfromActorInfo))
                (return false)))))
        (return false)
        (else
          (return false)))
      (else
        (CallFunction|BoxStrategyPrintStringError self "FindAndReserveResources" "Пришла мапа с доступными ресурсами для резерва, но она пустая.")
        (return false)))
    (else
      (return false))))

(fn ResetAllData
  (bind _returnvalue (Ability|GetAvatarActorfromActorInfo))
  (bind _returnvalue_2 (AI|GetAIController _returnvalue))
  (Utilities|FlowControl|Sequence
    (:then_0
      (Utilities|IsValid (Variables|Reserved|GetReservedResourceOnGround)
        (:Is%20Valid
          (Game|UnbindEventfromOnDestroyed (Variables|Reserved|GetReservedResourceOnGround) (EventDispatchers|CreateEvent :!event Custom|Event_ResourceWasDestroyed)))))
    (:then_1
      (Utilities|IsValid (Variables|AbilitySettings|GetMyTask)
        (:Is%20Valid
          (EventDispatchers|UnbindEventfromOnTaskWasCanceled (Variables|AbilitySettings|GetMyTask) (EventDispatchers|CreateEvent :!event Custom|Event_TaskWasCanceled)))))
    (:then_2
      (Utilities|IsValid (Ability|GetAvatarActorfromActorInfo)
        (:Is%20Valid
          (Collision|UnbindEventfromOnActorBeginOverlap (.AsCharacter (Utilities|Casting|CastToCharacter _returnvalue)) (EventDispatchers|CreateEvent :!event Custom|Event_CharacterOverlapSomething))
          (Utilities|IsValid _returnvalue_2
            (:Is%20Valid
              (AI|Navigation|StopMovement _returnvalue_2))))))
    (:then_3
      (Variables|Reserved|SetReservedAmount 0)
      (Variables|Reserved|SetReservedResourceOnGround 0)
      (Variables|AbilitySettings|SetMyTask 0))
    (:then_4
      (CallFunction|RemoveMeshfromCharacter))
    (:then_5
      (Utilities|Time|ClearandInvalidateTimerbyHandle (Variables|Default|GetEndingTimer)))))

(fn IsResourceNear
  (return (>= (+ (Variables|AbilitySettings|GetAcceptableRadius) 3e+01) (Math|Vector|VectorLength (- (Transformation|GetActorLocation (Variables|Reserved|GetReservedResourceOnGround)) (Transformation|GetActorLocation (Ability|GetAvatarActorfromActorInfo)))))))

(fn SaveReservedData
  (params (ReservedResourceOnGround :type BP%20Pickable%20Item%20Base%20Object%20Reference) (ReservedAmount :type Integer) (ReservedResourceData :type Box%20Strategy%20Product%20Data%20Base%20Object%20Reference))
  (Variables|Reserved|SetReservedAmount ReservedAmount)
  (Variables|Reserved|SetReservedResourceOnGround ReservedResourceOnGround)
  (Variables|Reserved|SetReservedResourceData ReservedResourceData))

(fn AddMeshtoCharacter
  (bind _aspickable_item_data_base (Utilities|Casting|CastToPickableItemData_Base (Variables|Reserved|GetReservedResourceData))
    (:then
      (LocalVariables|SetLocal_PureResourceData _aspickable_item_data_base)
      (bind _returnvalue (Utilities|LoadAssetBlocking (Variables|/Script/BoxStrategy.PickableItemData_Base|GetItemMesh (LocalVariables|GetLocal_PureResourceData))))
      (bind _asstatic_mesh (Utilities|Casting|CastToStaticMesh _returnvalue)
        (:then
          (LocalVariables|SetLocal_StaticMesh _asstatic_mesh)
          (Utilities|FlowControl|Sequence
            (:then_0
              (bind _returnvalue_2 (Game|AddComponentbyClass (Ability|GetAvatarActorfromActorInfo) "/Script/Engine.StaticMeshComponent" false))
              (Variables|Default|SetResourceStaticMeshComponent _returnvalue_2)
              (Collision|SetCollisionEnabled (Variables|Default|GetResourceStaticMeshComponent) "NoCollision")
              (Components|StaticMesh|SetStaticMesh (Variables|Default|GetResourceStaticMeshComponent) (LocalVariables|GetLocal_StaticMesh))
              (Transformation|SetRelativeScale3D (Variables|Default|GetResourceStaticMeshComponent) "0.500000,0.500000,0.250000")
              (bind _asbp_unit_character (Utilities|Casting|CastToBP_Unit_Character (Ability|GetAvatarActorfromActorInfo))
                (:then
                  (Default|EventAddComponentforDrug _asbp_unit_character (Variables|Default|GetResourceStaticMeshComponent)))
                (:CastFailed
                  (CallFunction|BoxStrategyPrintStringError self "AddMeshToRobot" "Cannot Cast to BP_Unit_character"))))
            (:then_1
              (bind _returnvalue_3 (Utilities|LoadAssetBlocking (Variables|/Script/BoxStrategy.PickableItemData_Base|GetItemMaterial (LocalVariables|GetLocal_PureResourceData))))
              (bind _asmaterial (Utilities|Casting|CastToMaterial _returnvalue_3)
                (:then
                  (Rendering|Material|SetMaterial (Variables|Default|GetResourceStaticMeshComponent) 0 _asmaterial))
                (:CastFailed
                  (bind _asmaterial_instance (Utilities|Casting|CastToMaterialInstance _returnvalue_3))
                  (Rendering|Material|SetMaterial (Variables|Default|GetResourceStaticMeshComponent) 0 _asmaterial_instance))))))
        (:CastFailed
          (return))))
    (:CastFailed
      (return))))

(fn RemoveMeshfromCharacter
  (bind _returnvalue (Ability|GetAvatarActorfromActorInfo))
  (Utilities|IsValid (Variables|Default|GetResourceStaticMeshComponent)
    (:Is%20Valid
      (Utilities|IsValid _returnvalue
        (:Is%20Valid
          (bind _asbp_unit_character (Utilities|Casting|CastToBP_Unit_Character _returnvalue))
          (Default|EventRemoveComponentforDrug _asbp_unit_character (Variables|Default|GetResourceStaticMeshComponent))
          (Variables|Default|SetResourceStaticMeshComponent 0))))))

(fn RespawnResourceNearRobot
  (bind _returnvalue (Ability|GetAvatarActorfromActorInfo))
  (if (> (Variables|Taken|GetTakenResourceAmount) 0)
    (Utilities|IsValid (Variables|Reserved|GetReservedResourceData)
      (:Is%20Valid
        (bind _returnvalue_2 (CallFunction|RecalculatetoGridPosition (+ (* (Transformation|GetActorForwardVector _returnvalue) 1.5e+02) (Transformation|GetActorLocation _returnvalue)) 5e+01))
        (bind (_outhit _returnvalue_3) (Collision|LineTraceByChannel (+ _returnvalue_2 "0.000000,0.000000,100.000000") (+ _returnvalue_2 "0.000000,0.000000,-1000.000000") "TraceTypeQuery1" false 0 "None"))
        (if _returnvalue_3
          (bind _returnvalue_4 (CallFunction|RecalculatetoGridPosition (.Location (Collision|BreakHitResult _outhit)) 5e+01))
          (Game|SpawnActorfromClass "/Game/BoxStrategy/Framework/GameObjects/Items/BP_ItemActor_PureResource.BP_ItemActor_PureResource_C" (Math|Transform|MakeTransform _returnvalue_4) "Undefined" "MultiplyWithRoot" 0 (Variables|Taken|GetTakenResourceAmount) (.AsPickable%20Item%20Data%20Base (Utilities|Casting|CastToPickableItemData_Base (Variables|Reserved|GetReservedResourceData))) 0)
          (else
            (CallFunction|BoxStrategyPrintStringError self "RespawnResourceNearRobot" "Невозможно найти место для ресурса.")))
        (Variables|Reserved|SetReservedAmount 0)
        (Variables|Reserved|SetReservedResourceData 0)))))

(fn TakeResourcefromItemonGround
  (Game|UnbindEventfromOnDestroyed (Variables|Reserved|GetReservedResourceOnGround) (EventDispatchers|CreateEvent :!event Custom|Event_ResourceWasDestroyed))
  (bind _takenamount (Default|TakeItemAmount (Variables|Reserved|GetReservedResourceOnGround) (Variables|Reserved|GetReservedAmount) (Ability|GetAvatarActorfromActorInfo)))
  (Variables|Taken|SetTakenResourceAmount _takenamount)
  (Variables|Reserved|SetReservedResourceOnGround 0)
  (Variables|Reserved|SetReservedAmount 0))

(fn IsUnitOverlappingTaskActor
  (return (Collision|IsOverlappingActor (Ability|GetAvatarActorfromActorInfo) (Default|GetTaskOwnerActor (Variables|AbilitySettings|GetMyTask)) :!class /Script/Engine.Actor)))

(fn DeliverResourcestoTaskandEndAbility
  (Default|DeliverResources (Variables|AbilitySettings|GetMyTask) (Utilities|Map|MakeMap (Variables|Reserved|GetReservedResourceData) (Variables|Taken|GetTakenResourceAmount)) (Ability|GetAvatarActorfromActorInfo))
  (Ability|EndAbility))