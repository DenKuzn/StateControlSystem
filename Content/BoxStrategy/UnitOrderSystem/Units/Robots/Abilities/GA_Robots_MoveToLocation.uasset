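; Gameplay ability that moves a robot unit's pawn to a target location in the box strategy unit order system.
; On activation it runs AI MoveTo toward the location read from the ability's BP_UOAS_Location settings and ends on success.
; On failure it waits a tick and ends only if the AI controller is not moving, otherwise leaving the ability active.
; Both outcomes print debug strings.
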(event Ability|EventActivateAbility
  (AI|AIMoveTo (.AsPawn (Utilities|Casting|CastToPawn (Ability|GetAvatarActorfromActorInfo))) (Variables|/Game/BoxStrategy/UnitOrderSystem/Units/Robots/Settings/BP_UOAS_Location.BP_UOAS_Location_C|GetLocation (.AsBP%20UOAS%20Location (Utilities|Casting|CastToBP_UOAS_Location (Class|UnitOrderGameplayAbility|GetMyAbilitySettings)))) 0 5.0 false
    (:OnSuccess
      (Development|PrintString "Success")
      (Ability|EndAbility :!label _label))
    (:OnFail
      (Development|PrintString "Fail")
      (Utilities|FlowControl|DelayUntilNextTick)
      (if (Utilities|Enum|NotEqual(Enum) (Class|AIController|GetMoveStatus (AI|GetAIController (Ability|GetAvatarActorfromActorInfo))) "Moving")
        (goto _label)))))