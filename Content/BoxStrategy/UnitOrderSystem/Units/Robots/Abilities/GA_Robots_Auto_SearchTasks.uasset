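; Gameplay ability that lets robot units automatically search for work from the player's task manager.
; On activation it finds BP_TaskManagerComponent on the player state and requests a task, registering as a waiting object if none is assigned and deregistering when it ends.
; An assigned task is wrapped in a task receiver and issued as a unit order that clears the order list, with its ability tag mapped from the task type.
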(event Ability|EventActivateAbility
  ;[1 0.2599 0 0.308 12] Если компонент задачи не найден, то абилка просто висит в памяти, пока ее не отключит Unit Control Ability Component
  (Utilities|CheckTaskManagerComponent
    (:then
      (bind _returnvalue (Class|TaskManagerComponent|TryAssignTasktoUnit (Variables|Default|GetTaskManagerComponent) self))
      (if (not _returnvalue)
        (Class|TaskManagerComponent|AddforTaskWaitingObject (Variables|Default|GetTaskManagerComponent) self)))))

(event Ability|EventOnEndAbility
  (params (bWasCancelled :type Boolean))
  (Utilities|IsValid (Variables|Default|GetTaskManagerComponent)
    (:Is%20Valid
      (Class|TaskManagerComponent|RemoveTaskWaitingObject (Variables|Default|GetTaskManagerComponent) self))))

(fn TryGetNewTask)

(fn GetOwningActor
  (return (Ability|GetAvatarActorfromActorInfo)))

(fn GetUnitSubtypeTag
  (return (Class|UnitOrderGameplayAbility|GetMyUnitSubtypeTag)))

(fn NewTaskAssigned
  (params (NewTask :type Box%20Strategy%20Unit%20Task%20Object%20Reference))
  (bind _returnvalue (Game|ConstructObjectfromClass "/Game/BoxStrategy/UnitOrderSystem/Units/Robots/Settings/BP_UOAS_TaskReceiver.BP_UOAS_TaskReceiver_C" NewTask))
  (Class|UnitOrderAbilitySystemComponent|ExecuteNewUnitOrder (Class|UnitOrderGameplayAbility|GetUnitOrderAbilitySystemComponent) _returnvalue (CallFunction|GetAbilityTagfromTaskTagRobotsBridge (Default|GetTaskTypeTag NewTask)) true))