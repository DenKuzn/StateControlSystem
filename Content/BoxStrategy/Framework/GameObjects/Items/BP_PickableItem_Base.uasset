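; Base actor for a pickable resource item in the strategy game, configured from product data that sets its mesh, dynamic material and clamped stack amount.
; Units reserve amounts in a per-reserver map, pruned of invalid reservers; non-stackable items allow only one reservation.
; Taking releases the taker's reservation, deducts the amount and destroys the actor at zero.
; An item information widget shows only while the item is selected.
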(event ObjectWasSeleceted(StateControlInteract)
  (Rendering|SetVisibility (Variables|Default|GetWidget) true true))

(event ObjectWasDeseleceted(StateControlInteract)
  (Rendering|SetVisibility (Variables|Default|GetWidget) false true))

(event EventBeginPlay
  (Rendering|SetVisibility (Variables|Default|GetWidget) false true)
  (bind _aswbp_item_inforamtion (Utilities|Casting|CastToWBP_ItemInforamtion (UserInterface|GetUserWidgetObject (Variables|Default|GetWidget)))
    (:then
      (Default|EventSetNewItem _aswbp_item_inforamtion self))
    (:CastFailed
      (CallFunction|BoxStrategyPrintStringError self "BeginPlay" "Widget ItemInformation invalid"))))

(fn ConstructionScript
  (bind _new_productdata (Variables|Default|GetNew_ProductData))
  (bind _new_productdata_2 (Variables|Default|GetNew_ProductData))
  (bind _itemmaterial (Variables|/Script/BoxStrategy.PickableItemData_Base|GetItemMaterial _new_productdata_2))
  (bind _itemmesh (Variables|/Script/BoxStrategy.PickableItemData_Base|GetItemMesh _new_productdata))
  (Utilities|IsValid (Variables|Default|GetNew_ProductData)
    (:Is%20Valid
      (Utilities|FlowControl|Sequence
        (:then_0
          (if (Utilities|IsValidSoftObjectReference _itemmesh)
            (bind _returnvalue (Utilities|LoadAssetBlocking _itemmesh))
            (Utilities|IsValid (.AsStatic%20Mesh (Utilities|Casting|CastToStaticMesh _returnvalue))
              (:Is%20Valid
                (Components|StaticMesh|SetStaticMesh (Variables|Default|GetSM_ResourceBox) (.AsStatic%20Mesh (Utilities|Casting|CastToStaticMesh _returnvalue)))))))
        (:then_1
          (if (Variables|/Script/BoxStrategy.PickableItemData_Base|GetbCanStock (Variables|Default|GetNew_ProductData))
            (Private|SetNewItemAmount (Variables|Default|GetCurrentItemAmount))
            (else
              (Private|SetNewItemAmount 1))))
        (:then_2
          (if (Utilities|IsValidSoftObjectReference _itemmaterial)
            (bind _returnvalue_2 (Utilities|LoadAssetBlocking _itemmaterial))
            (bind _asmaterial (Utilities|Casting|CastToMaterial _returnvalue_2)
              (:then
                (bind _returnvalue_3 (Rendering|Material|CreateDynamicMaterialInstance _asmaterial "None" "None" :!class /Script/Engine.KismetMaterialLibrary))
                (Rendering|Material|SetMaterial (Variables|Default|GetSM_ResourceBox) 0 _returnvalue_3))
              (:CastFailed
                (bind _asmaterial_instance (Utilities|Casting|CastToMaterialInstance _returnvalue_2))
                (bind _returnvalue_4 (Rendering|Material|CreateDynamicMaterialInstance _asmaterial_instance "None" "None" :!class /Script/Engine.KismetMaterialLibrary))
                (Rendering|Material|SetMaterial (Variables|Default|GetSM_ResourceBox) 0 _returnvalue_4)))))))))

(fn SetNewItemAmount
  (params (Value :type Integer))
  (Variables|Default|SetCurrentItemAmount (Math|Integer|Clamp(Integer) Value 0 (Variables|/Script/BoxStrategy.PickableItemData_Base|GetMaxStock (Variables|Default|GetNew_ProductData)))))

(fn ReserveItemAmount
  (params (WhoReserves :type Object%20Object%20Reference) (AmountForReserve :type Integer))
  (if (not (.ReturnValue (Utilities|Map|Find (Variables|Default|GetReservedResources) WhoReserves)))
    (Utilities|IsValid (Variables|Default|GetNew_ProductData)
      (:Is%20Valid
        (bind (_can _availableamount) (Public|CanReservewithValidation))
        (LocalVariables|SetLocal_AvailableResourceAmountForReserve _availableamount)
        (if _can
          (if (<= AmountForReserve (LocalVariables|GetLocal_AvailableResourceAmountForReserve))
            (Utilities|Map|Add (Variables|Default|GetReservedResources) WhoReserves AmountForReserve)
            (Default|CallOnDataChanged)
            (return AmountForReserve)
            (else
              (Development|PrintString "Error: Попытка зарезервировать ресурс больше, чем есть свободное количество.")
              (Utilities|Map|Add (Variables|Default|GetReservedResources) WhoReserves (LocalVariables|GetLocal_AvailableResourceAmountForReserve))
              (Default|CallOnDataChanged)
              (return (LocalVariables|GetLocal_AvailableResourceAmountForReserve))))
          (else
            (Development|PrintString "Error: Нельзя зарезервировать ресурс.")
            (return 0))))
      (:Is%20Not%20Valid
        (CallFunction|BoxStrategyPrintStringError self "ReserveItemAmount" "ProductData invalid")
        (return 0)))
    (else
      (Development|PrintString "Error: Попытка зарезервировать ресурс кем-то, кто уже зарезервировал себе ресурс.")
      (return 0))))

(fn CanReservewithValidation
  (Private|ValidateAllResourceReservers)
  (bind (_can _availableamount) (Public|CanReserve))
  (return _can _availableamount))

(fn ValidateAllResourceReservers
  (bind _keys (Utilities|Map|Keys (Variables|Default|GetReservedResources)))
  (bind _output_get (LocalVariables|SetLocal_Reservers _keys))
  (for _array_element _output_get
    (if (not (Utilities|IsValid _array_element))
      (Utilities|Map|Remove (Variables|Default|GetReservedResources) _array_element)
      (LocalVariables|SetbDataChanged true)))
  (if (LocalVariables|GetbDataChanged)
    (Default|CallOnDataChanged))
  (return))

(fn CanReserve
  (if (> (Variables|Default|GetCurrentItemAmount) 0)
    (Utilities|IsValid (Variables|Default|GetNew_ProductData)
      (:Is%20Valid
        (bind _keys (Utilities|Map|Keys (Variables|Default|GetReservedResources)))
        (LocalVariables|SetLocal_WhoReservedResources _keys)
        (if (> (Utilities|Array|Length (LocalVariables|GetLocal_WhoReservedResources)) 0)
          (if (Variables|/Script/BoxStrategy.PickableItemData_Base|GetbCanStock (Variables|Default|GetNew_ProductData))
            (LocalVariables|SetLocal_ReservedAmount (CallFunction|GetReservedAmount))
            (return (< (LocalVariables|GetLocal_ReservedAmount) (Variables|Default|GetCurrentItemAmount)) (select (< (LocalVariables|GetLocal_ReservedAmount) (Variables|Default|GetCurrentItemAmount)) (- (Variables|Default|GetCurrentItemAmount) (LocalVariables|GetLocal_ReservedAmount)) 0))
            (else
              (return false 0)))
          (else
            (return true (Variables|Default|GetCurrentItemAmount)))))
      (:Is%20Not%20Valid
        (CallFunction|BoxStrategyPrintStringError self "CanReserve" "Product Data invalind")
        (return false 0)))
    (else
      (CallFunction|BoxStrategyPrintStringError self "CanReserve" "CurrentItemAmount <= 0. Amount = " (Utilities|String|ToString(Integer) (Variables|Default|GetCurrentItemAmount)))
      (return false 0))))

(fn TakeItemAmount
  (params (TakenItemAmount :type Integer) (WhoTaked :type Object%20Object%20Reference))
  (bind _reservedresources (Variables|Default|GetReservedResources))
  (bind (_value _returnvalue) (Utilities|Map|Find _reservedresources WhoTaked))
  (Private|ValidateAllResourceReservers)
  (if _returnvalue
    (LocalVariables|SetLocal_ReservedAmount _value)
    (Utilities|Map|Remove (Variables|Default|GetReservedResources) WhoTaked)
    (if (== (LocalVariables|GetLocal_ReservedAmount) TakenItemAmount)
      (if (>= (- (Variables|Default|GetCurrentItemAmount) TakenItemAmount) 0) ; Это нужно в большей степени для выявления ошибок.\nА вообще можно было просто в кламп и выдать.
        (LocalVariables|SetLocal_canTakeAmount TakenItemAmount)
        (else
          (Development|PrintString "Error: Юнит пытается взять больше ресурсов, чем доступно в итеме.")
          (bind (_can _availableamount) (Public|CanReserve :!label _label))
          (if _can
            (LocalVariables|SetLocal_canTakeAmount (Math|Integer|Clamp(Integer) _availableamount 0 TakenItemAmount))
            (else
              (Development|PrintString "Error: В итеме нет доступных ресурсов для взятия.")
              (return 0)))))
      (else
        (Development|PrintString "Error: Юнит резервировал одно значение, но теперь запрашивает новое по какой-то причине.")
        (goto _label)))
    (else
      (goto _label)))
  (Variables|Default|SetCurrentItemAmount (- (Variables|Default|GetCurrentItemAmount) (LocalVariables|GetLocal_canTakeAmount)))
  (if (== (Variables|Default|GetCurrentItemAmount) 0)
    (Actor|DestroyActor)
    (else
      (Default|CallOnDataChanged)))
  (return (LocalVariables|GetLocal_canTakeAmount)))

(fn CancelItemAmountReservation
  (params (WhoReserves :type Object%20Object%20Reference))
  (bind _returnvalue (Utilities|Map|Remove (Variables|Default|GetReservedResources) WhoReserves))
  (if _returnvalue
    (Default|CallOnDataChanged)
    (return)
    (else
      (Development|PrintString "Error: Попытка снять резервацию кем-то, кто не был в резерве")
      (return))))

(fn GetItemType
  (return (Variables|/Script/BoxStrategy.BoxStrategyProductData_Base|GetMainTypeTag (Variables|Default|GetNew_ProductData))))

(fn GetItemName
  (return (.MainName (Utilities|Struct|BreakObjectDescription (Variables|/Script/BoxStrategy.BoxStrategyProductData_Base|GetDescription (Variables|Default|GetNew_ProductData))))))

(fn GetCurrentAmount
  (return (Variables|Default|GetCurrentItemAmount)))

(fn GetReservedAmount
  (bind _keys (Utilities|Map|Keys (Variables|Default|GetReservedResources)))
  (for _array_element _keys
    (Utilities|IsValid _array_element
      (:Is%20Valid
        (LocalVariables|SetLocal_ReservedAmount (+ (LocalVariables|GetLocal_ReservedAmount) (.Value (Utilities|Map|Find (Variables|Default|GetReservedResources) _array_element)))))))
  (return (LocalVariables|GetLocal_ReservedAmount)))