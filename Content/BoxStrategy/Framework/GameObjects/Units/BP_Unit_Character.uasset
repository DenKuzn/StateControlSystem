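; Unit character for the BoxStrategy game, with selection markers and a hand weapon.
; On BeginPlay it hides both markers, links the Niagara bullet effect component to the hand weapon component and equips a test rifle.
; StateControlInteractComponent selection events toggle the markers, showing the move-location mark only if the AI unit controller reports Moving.
; Also contains an AI controller validity macro and unconnected asset-loading test nodes.
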(event EventBeginPlay
  (Rendering|SetVisibility (Variables|Default|GetMoveLocationMark) false false)
  (Class|BoxStrategyHandWeaponComponent|InitializeHandWeaponComponent (Variables|Default|GetBoxStrategyHandWeapon) 0 0 (Variables|Default|GetNiagara))
  (Class|BoxStrategyHandWeaponComponent|EquipNewWeapon (Variables|Default|GetBoxStrategyHandWeapon) "/Game/BoxStrategy/DataAssets/Items/Weapons/DA_Rifle_Test.DA_Rifle_Test"))

(event ObjectWasDeseleceted(StateControlInteractComponent)
  ;[0 0.7406 1] Select Unit States
  (Rendering|SetVisibility (Variables|Default|GetSelectMark) false false))

(event ObjectWasSeleceted(StateControlInteractComponent)
  ;[0 0.7406 1] Select Unit States
  (Rendering|SetVisibility (Variables|Default|GetSelectMark) true false)
  (if (Utilities|Enum|Equal(Enum) (Class|AIController|GetMoveStatus (Class|BoxStrategyUnitCharacter|GetAIUnitController)) "Moving")
    (Rendering|SetVisibility (Variables|Default|GetMoveLocationMark) true false)))

(fn ConstructionScript)