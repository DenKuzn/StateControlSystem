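; Robot factory building Blueprint for a strategy game, handling the switch from under construction to finished and selection feedback.
; When construction ends, it applies a blue base material, enables the StateControlInteractComponent, makes the Box block the Camera channel and destroys its widget.
; The component's selected and deselected events show and hide a Plane, but only while interaction is enabled.
; No robot production logic is present in these graphs.
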(event ObjectWasSeleceted(StateControlInteractComponent)
  (if (Class|StateControlInteractComponent|IsInteractionEnabled (Variables|Default|GetStateControlInteractComponent))
    (Rendering|SetVisibility (Variables|Default|GetPlane) true false)))

(event ObjectWasDeseleceted(StateControlInteractComponent)
  (if (Class|StateControlInteractComponent|IsInteractionEnabled (Variables|Default|GetStateControlInteractComponent))
    (Rendering|SetVisibility (Variables|Default|GetPlane) false false)))

(event EventConstructionEnded
  (Rendering|Material|SetMaterial (Variables|Default|GetBaseBuildingMesh) 0 "/Game/TestContent/Materials/TEST_MI_BlueColor_Base.TEST_MI_BlueColor_Base")
  (Class|StateControlInteractComponent|SetInteraction (Variables|Default|GetStateControlInteractComponent) true)
  (Collision|SetCollisionResponsetoChannel (Variables|Default|GetBox) "ECC_Camera" "ECR_Block")
  (Components|DestroyComponent (Variables|Default|GetWidget)))

(fn ConstructionScript)