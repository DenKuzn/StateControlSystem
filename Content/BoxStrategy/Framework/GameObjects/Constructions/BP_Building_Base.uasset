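; Base building actor for a strategy game, covering placement preview, timed construction and the switch to a working state.
; An enum state gates placement: the preview follows new positions and tints a dynamic material by Box overlap checks.
; Placing enables blocking collision, enlarges the Box until completion and starts ProductionSystemComponent, whose delegates drive the progress widget.
; Derived classes override ConstructionEnded; rotation is only a print stub.
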(event Custom|Event_NewPosition
  (params (NewPosition :type Vector))
  (bind _returnvalue (+ NewPosition "0.000000,0.000000,1.000000"))
  ;[1 1 1] TODO: Переписать состояния с енума на классы и создать возможность подключения состояний по этапам здания.
  ;;[0.2504 0.07565 0.5719 0.337] Searching New Position.
  (Utilities|CheckCurrentState "SearchingPlace"
    (:true
      (if (not (Utilities|Operators|EqualEqual (Transformation|GetActorLocation) _returnvalue 1.0))
        (Transformation|SetActorLocation _returnvalue false false)
        (Class|MyExtensionBlueprintFunctionLibrary|UpdateComponentOverlaps (Variables|Default|GetBox)))
      (CallFunction|ChangeAvailabilityColor))
    (:false
      (Utilities|ErrorwithState "Event_NewPosition"))))

(event Custom|Event_PlaceBuildHere
  ;[1 1 1] TODO: Переписать состояния с енума на классы и создать возможность подключения состояний по этапам здания.
  (if (CallFunction|IsCanBuildHere)
    (Utilities|CheckCurrentState "SearchingPlace"
      (:true
        (Class|BoxStrategyBuilding|SetBuildingState "Constructing")
        (CallFunction|SetBuildingonGround)
        (CallFunction|ShowWidgetandSetSettings)
        (CallFunction|StartBuildingProduction))
      (:false
        (Utilities|ErrorwithState "Event_PlaceBuildHere")
        (Actor|DestroyActor)))
    (else
      (CallFunction|BoxStrategyPrintStringError self "Event_PlaceBuildHere" "Cannot Build Here.")
      (Actor|DestroyActor))))

(event Custom|Event_ProductionProgressUpdated
  (params (NormalizedProgress :type Float%20%28single-precision%29))
  ;[1 1 1] TODO: Переписать состояния с енума на классы и создать возможность подключения состояний по этапам здания.
  (Default|EventConstructionSetPercent (Variables|Default|GetMyWidgetInformation) NormalizedProgress))

(event Custom|Event_CancelConstruction
  (params (AreYouAskedThePlayer? :type Boolean))
  (if AreYouAskedThePlayer?
    (if (Utilities|Enum|Equal(Enum) (Class|BoxStrategyBuilding|GetBuildingState) "Constructing")
      (CallFunction|ResetDelegatesFomBuildingProduction))
    (Actor|DestroyActor)
    (else
      (Development|PrintString "Error: ВНИМАНИЕ. СПРОСИТЕ ЗАРАНЕЕ, ПОТОМУ ЧТО ЭТА ФФУНКЦИЯ НЕ СПРАШИВАЕТ."))))

(event Custom|Event_NewRotation
  (params (Left :type Boolean))
  ;[1 1 1] TODO: Переписать состояния с енума на классы и создать возможность подключения состояний по этапам здания.
  ;;[0.2504 0.07565 0.5719 0.337] Searching New Position.
  (Development|PrintString (Utilities|String|ToString(Boolean) Left)))

(event Custom|Event_InitializeBuilding
  (params (NewConstructionData :type Construction%20Data%20Base%20Object%20Reference))
  (Class|BoxStrategyBuilding|SetBuildingData NewConstructionData)
  (Utilities|CheckBuildingData)
  (CallFunction|SetupConstructMaterialforBuilding)
  (Class|BoxStrategyBuilding|SetBuildingState "SearchingPlace")
  (CallFunction|SetupWidget))

(event Custom|ConstructionEnded)

(event Custom|Event_ConstructionCompleted
  ;[1 1 1] TODO: Переписать состояния с енума на классы и создать возможность подключения состояний по этапам здания.
  (Class|BoxStrategyBuilding|SetBuildingState "Working")
  (Default|EventConstructionSetPercent (Variables|Default|GetMyWidgetInformation) 1.0)
  (Components|Box|SetBoxExtent (Variables|Default|GetBox) (- (Variables|/Script/Engine.BoxComponent|GetBoxExtent (Variables|Default|GetBox)) (Variables|Default|GetBoxExtend)) true)
  (CallFunction|ResetDelegatesFomBuildingProduction)
  (CallFunction|ConstructionEnded))

(fn ConstructionScript)

(fn IsCanBuildHere
  (return (not (Utilities|Array|IsValidIndex (Collision|GetOverlappingActors (Variables|Default|GetBox) "/Script/Engine.Actor" :!class /Script/Engine.PrimitiveComponent)))))

(fn ChangeAvailabilityColor
  (bind _constructmaterial_instance (Variables|Default|GetConstructMaterial_Instance))
  (Utilities|IsValid _constructmaterial_instance
    (:Is%20Valid
      (Rendering|Material|SetVectorParameterValue _constructmaterial_instance "Color" (select (CallFunction|IsCanBuildHere) (Variables|Default|GetColor_Available) (Variables|Default|GetColor_NotAvailable)) :!class /Script/Engine.MaterialInstanceDynamic))))

(fn SetupConstructMaterialforBuilding
  (bind _returnvalue (Rendering|Material|CreateDynamicMaterialInstance "/Game/TestContent/Materials/TEST_M_SimpleColorWithAlpha_Base.TEST_M_SimpleColorWithAlpha_Base" "None" "None" :!class /Script/Engine.KismetMaterialLibrary))
  (bind _output_get (Variables|Default|SetConstructMaterial_Instance _returnvalue))
  (Rendering|Material|SetMaterial (Variables|Default|GetBaseBuildingMesh) 0 _output_get))

(fn SetupWidget
  (bind _output_get (Variables|Default|SetMyWidgetInformation (.AsWBP%20Construction%20Template%20Information (Utilities|Casting|CastToWBP_ConstructionTemplateInformation (UserInterface|GetUserWidgetObject (Variables|Default|GetWidget))))))
  (Variables|/Game/BoxStrategy/Widgets/InObjectWidgets/WBP_ConstructionTemplateInformation.WBP_ConstructionTemplateInformation_C|SetMyBossConstructionTemplate _output_get self))

(fn SetBuildingonGround
  (bind _returnvalue (Transformation|GetActorLocation))
  (bind (_x _y _z) (Math|Vector|BreakVector _returnvalue))
  (Transformation|SetActorLocation (Math|Vector|MakeVector _x _y (- _z 1.0)) false false)
  (Rendering|Material|SetVectorParameterValue (Variables|Default|GetConstructMaterial_Instance) "Color" (Variables|Default|GetColor_Placed) :!class /Script/Engine.MaterialInstanceDynamic)
  (Collision|SetCollisionObjectType (Variables|Default|GetBaseBuildingMesh) "ECC_WorldStatic")
  (Collision|SetCollisionResponsetoAllChannels (Variables|Default|GetBaseBuildingMesh) "ECR_Block")
  (Components|Box|SetBoxExtent (Variables|Default|GetBox) (+ (Variables|/Script/Engine.BoxComponent|GetBoxExtent (Variables|Default|GetBox)) (Variables|Default|GetBoxExtend)) true))

(fn ShowWidgetandSetSettings
  (Rendering|SetVisibility (Variables|Default|GetWidget) true true)
  (Default|EventConstructionSetPercent (Variables|Default|GetMyWidgetInformation) 0.0))

(fn StartBuildingProduction
  (EventDispatchers|BindEventtoOnProductionCompleted (Variables|Default|GetProductionSystemComponent) (EventDispatchers|CreateEvent :!event Custom|Event_ConstructionCompleted))
  (EventDispatchers|BindEventtoOnProductionProgressUpdated (Variables|Default|GetProductionSystemComponent) (EventDispatchers|CreateEvent :!event Custom|Event_ProductionProgressUpdated))
  (Class|ProductionSystemComponent|AddNextProduct (Variables|Default|GetProductionSystemComponent) (Variables|Default|GetBoxStrategyConstructionData))
  (Class|ProductionSystemComponent|ActivateProduction (Variables|Default|GetProductionSystemComponent)))

(fn ResetDelegatesFomBuildingProduction
  (EventDispatchers|UnbindEventfromOnProductionCompleted (Variables|Default|GetProductionSystemComponent) (EventDispatchers|CreateEvent :!event Custom|Event_ConstructionCompleted))
  (EventDispatchers|UnbindEventfromOnProductionProgressUpdated (Variables|Default|GetProductionSystemComponent) (EventDispatchers|CreateEvent :!event Custom|Event_ProductionProgressUpdated)))